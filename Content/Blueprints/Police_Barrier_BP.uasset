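; Police barrier actor that adds stress to the first-person player and changes its appearance when overlapped.
; On overlap, it sets the character's stress damage, calls its stress bar update and destroys the Box component.
; Separate sequence branches swap the barrier mesh to a cube and spawn a louder audio component once.
; Only the stress and Box branch depends on the character cast, so any overlapping actor triggers the mesh and sound.
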(event Collision|EventActorBeginOverlap
  (params (OtherActor :type Actor%20Object%20Reference))
  (Utilities|FlowControl|Sequence
    (:then_0
      (bind _asfirst_person_character (Utilities|Casting|CastToFirstPersonCharacter OtherActor))
      (Variables|/Game/FirstPersonBP/Blueprints/FirstPersonCharacter.FirstPersonCharacter_C|SetDamage_Stress _asfirst_person_character 1e+01)
      (Default|StressBar _asfirst_person_character)
      (Components|DestroyComponent (Variables|Default|GetBox)))
    (:then_1
      (Components|StaticMesh|SetStaticMesh (Variables|Default|GetPolice_Barrier) "/Game/Models/1M_Cube.1M_Cube"))
    (:then_2
      (Utilities|FlowControl|DoOnce false
        (:Completed
          (bind _returnvalue (AddComponent|AddAudioComponent false))
          (Audio|Components|Audio|SetVolumeMultiplier _returnvalue 2.0 :!class /Script/Engine.AudioComponent))))))

(fn ConstructionScript)